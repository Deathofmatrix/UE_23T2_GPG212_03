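; BP_FinishLine is a level-end trigger that records the player's completion time and loads the next level.
; Any overlap with its box plays a coin sound, then writes the character's minutes, seconds and milliseconds as an IntVector into the GameInstance's LevelTimes array before opening LevelToLoadName.
; The array index comes from the number following the level name's five-character prefix, minus one.
; BeginPlay caches the first-person character and logs all stored times.
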(event OnComponentBeginOverlap(Box)
  (params (OverlappedComponent :type Primitive%20Component%20Object%20Reference) (OtherActor :type Actor%20Object%20Reference) (OtherComp :type Primitive%20Component%20Object%20Reference) (OtherBodyIndex :type Integer) (bFromSweep :type Boolean) (SweepResult :type Hit%20Result%20Structure%20%28by%20ref%29))
  (bind _character_reference (Variables|Default|GetCharacter%20Reference))
  (Audio|SpawnSound2D "/Game/Audio/coin2.coin2" 1.0 1.0 0.0 0 true)
  (bind _returnvalue (Game|GetCurrentLevelName true))
  (bind _asbp_game_instance (Utilities|Casting|CastToBP_GameInstance (Game|GetGameInstance)))
  (Utilities|Array|SetArrayElem (Variables|/Game/Blueprints/BP_GameInstance.BP_GameInstance_C|GetLevelTimes _asbp_game_instance) (- (Math|Conversions|ToInteger(Byte) (Utilities|String|RightChop _returnvalue 5)) 1) (Utilities|Struct|MakeIntVector (Variables|/Game/FirstPerson/Blueprints/BP_FirstPersonCharacter.BP_FirstPersonCharacter_C|GetMinutes _character_reference) (Variables|/Game/FirstPerson/Blueprints/BP_FirstPersonCharacter.BP_FirstPersonCharacter_C|GetSeconds _character_reference) (Variables|/Game/FirstPerson/Blueprints/BP_FirstPersonCharacter.BP_FirstPersonCharacter_C|GetMilliseconds _character_reference)))
  (Game|OpenLevel(byName) (Variables|Default|GetlevelToLoadName)))

(event EventBeginPlay
  (bind _returnvalue (Actor|GetActorOfClass "/Game/FirstPerson/Blueprints/BP_FirstPersonCharacter.BP_FirstPersonCharacter_C"))
  (Variables|Default|SetCharacter%20Reference _returnvalue)
  (bind _asbp_game_instance (Utilities|Casting|CastToBP_GameInstance (Game|GetGameInstance)))
  (for _array_element (Variables|/Game/Blueprints/BP_GameInstance.BP_GameInstance_C|GetLevelTimes _asbp_game_instance)
    (Development|PrintString (Class|KismetStringLibrary|BuildStringIntVector "" "" _array_element) false)))

(fn ConstructionScript)
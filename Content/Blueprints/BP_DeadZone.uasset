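; Dead zone trigger actor that restarts the current level when its box is overlapped.
; On begin overlap it plays a lose sound, waits briefly, then reopens the level by its current name, with no check on the overlapping actor.
; The construction script toggles the plane's visibility from ShowPlane and scales both plane and box in X and Y by Size.
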(event OnComponentBeginOverlap(Box)
  (params (OverlappedComponent :type Primitive%20Component%20Object%20Reference) (OtherActor :type Actor%20Object%20Reference) (OtherComp :type Primitive%20Component%20Object%20Reference) (OtherBodyIndex :type Integer) (bFromSweep :type Boolean) (SweepResult :type Hit%20Result%20Structure%20%28by%20ref%29))
  (Audio|PlaySound2D "/Game/Audio/lose8.lose8" 1.0 1.0 0.0 0 0)
  (Utilities|FlowControl|Delay 1.5)
  (bind _returnvalue (Game|GetCurrentLevelName true))
  (Game|OpenLevel(byName) (Utilities|String|StringToName _returnvalue)))

(fn ConstructionScript
  (bind _size (Variables|Default|Getsize))
  (Rendering|SetVisibility (Variables|Default|GetPlane) (Variables|Default|GetshowPlane) false)
  (Transformation|SetRelativeScale3D (Variables|Default|GetPlane) (Math|Vector|MakeVector _size _size 1.0)))